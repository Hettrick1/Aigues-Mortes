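; Placement preview actor that shows a mesh with a green or red shadow decal, depending on whether it can be placed.
; The construction script limits a SceneCapture2D to the mesh, assigns MeshRef, fits the box collider to the mesh bounds and picks the decal material from CanBePlaced.
; ScaleDecalToMesh is an empty stub, and the event graph has no runtime logic.
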(fn `ChangeShadowColor`
  (params (CanBePlaced :type Boolean))
  (bind _shadow (`self.Shadow`))
  (if CanBePlaced
    (`DecalComponent.SetDecalMaterial` _shadow "/Game/Blueprint/ColoredShadows/MI_ShadowGreen.MI_ShadowGreen")
    (else
      (`DecalComponent.SetDecalMaterial` _shadow "/Game/Blueprint/ColoredShadows/MI_ShadowRed.MI_ShadowRed"))))

(fn `ScaleCollider`
  (bind _colider (`self.Colider`))
  (bind (_origin _boxextent) (`KismetSystemLibrary.GetComponentBounds` (`self.Mesh`)))
  (`SceneComponent.K2_SetRelativeLocation` _colider _origin false false)
  (`BoxComponent.SetBoxExtent` _colider _boxextent true))

(fn `ScaleDecalToMesh`)

(fn `UserConstructionScript`
  ;[1 1 1] SetupRenderCapture
  (`SceneCaptureComponent.ShowOnlyComponent` (`self.SceneCaptureComponent2D`) (`self.Mesh`))
  ;[1 1 1] ShityTofix
  (`StaticMeshComponent.SetStaticMesh` (`self.Mesh`) (`self.MeshRef`))
  (`self.ScaleCollider`)
  (`self.ChangeShadowColor` (`self.CanBePlaced`))
  (`self.ScaleDecalToMesh`))