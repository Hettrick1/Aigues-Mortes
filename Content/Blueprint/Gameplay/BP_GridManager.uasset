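; Grid manager actor that builds a ground-snapped grid of points within its bounds on BeginPlay and returns the nearest point to a given location.
; PopulateGrid lays out cell-spaced points, then CheckForGround box-traces each for "Floor"-tagged actors.
; Invalid points are removed, while valid ones take their height from a vertical line trace.
; GetNearestPoint linearly scans squared distances, and debug boxes can be toggled to show the grid.
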(event `ClearPoints`
  ;[1 1 1] Clear Grid Points
  (`KismetArrayLibrary.Array_Clear` (`self.gridPointsArray`))
  (`KismetArrayLibrary.Array_Clear` (`self.gridPointsToRemove`))
  (`KismetArrayLibrary.Array_Clear` (`self.isPointValid`))
  (`KismetArrayLibrary.Array_Clear` (`self.gridPointsToAdjust`))
  (`KismetSystemLibrary.FlushPersistentDebugLines`))

(event `StartStopDrawDebug`
  ;[1 1 1] Start / Stop draw grid debug
  (`/Engine/EditorBlueprintResources/StandardMacros.FlipFlop`
    (:`A`
      (`self.DebugDraw`))
    (:`B`
      (`KismetSystemLibrary.FlushPersistentDebugLines`))))

(event `PopulateGrid`
  (bind (_returnvalue_x _returnvalue_y _returnvalue_z) (`KismetMathLibrary.BreakVector` (`self.K2_GetActorLocation`)))
  (bind _returnvalue (/ (.x (`.BoxExtent` (`self.GetActorBounds` false true))) (`self.gridCellSize`)))
  (bind _returnvalue_2 (/ (.y (`.BoxExtent` (`self.GetActorBounds` false true))) (`self.gridCellSize`)))
  ;[1 1 1] Populate Grid
  (`self.ClearPoints`)
  (`KismetArrayLibrary.Array_Clear` (`self.gridPointsToRemove`))
  (for _index (range (* _returnvalue_2 -1) (+ _returnvalue_2 1))
    (for _index_2 (range (* _returnvalue -1) (+ _returnvalue 1))
      (`KismetArrayLibrary.Array_AddUnique` (`self.gridPointsArray`) (`KismetMathLibrary.MakeVector` (- _returnvalue_x (* _index_2 (`self.gridCellSize`))) (- _returnvalue_y (* _index (`self.gridCellSize`))) _returnvalue_z))))
  (`self.CheckForGround`)
  (`KismetArrayLibrary.Array_Clear` (`self.isPointValid`))
  (if (`self.showDebugGrid`)
    (`self.DebugDraw`)))

(event `DebugDraw`
  ;[1 1 1] Draw Grid Debug
  (for _array_element (`self.gridPointsArray`)
    (bind _returnvalue (`GameplayStatics.GetActorOfClass` "/Script/Engine.PlayerStart"))
    (`KismetSystemLibrary.DrawDebugBox` _array_element (`KismetMathLibrary.Conv_DoubleToVector` (* (`self.gridCellSize`) 0.5)) (struct :`R` 0.25572 :`G` 1.0 :`A` 1.0) (struct) 10000000000.0 2.0)
    (`KismetSystemLibrary.DrawDebugBox` _array_element (10.0 10.0 10.0) (struct :`R` 1.0 :`G` 0.01469 :`A` 1.0) (struct) 10000000000.0 2.0)))

(event `InvalidatePoint`
  (params (`Dimension 1` :type Integer) (NewItem :type "Vector Structure (by ref)"))
  ;[1 1 1] Invalidate outside points
  (if (not (`|GetArrayItem` (`self.isPointValid`) `Dimension 1`))
    (`KismetArrayLibrary.Array_AddUnique` (`self.gridPointsToRemove`) NewItem)))

(event `self.ReceiveBeginPlay`
  (`self.PopulateGrid`))

(event `CheckFloor`
  (params (Start :type "Vector Structure") (End :type "Vector Structure") (HalfSize :type "Vector Structure") (Index :type Integer))
  (bind _x (.x Start))
  (bind _y (.y Start))
  ;[1 1 1] Check Floor for each points
  (bind (_outhits _returnvalue) (`KismetSystemLibrary.BoxTraceMulti` Start End HalfSize (struct) "TraceTypeQuery2"))
  (if _returnvalue
    (for _array_element _outhits
      (if (`self.ActorHasTag` (`.HitActor` (`GameplayStatics.BreakHitResult` _array_element)) "Floor")
        (`KismetArrayLibrary.Array_Set` (`self.isPointValid`) Index true true)
        (bind (_outhit _returnvalue_2) (`KismetSystemLibrary.LineTraceSingle` (`KismetMathLibrary.MakeVector` _x _y 1000.0) (`KismetMathLibrary.MakeVector` _x _y -1000.0) "TraceTypeQuery3"))
        (if _returnvalue_2
          (`KismetArrayLibrary.Array_AddUnique` (`self.gridPointsToAdjust`) (`.ImpactPoint` (`GameplayStatics.BreakHitResult` _outhit)))
          (else
            (`KismetArrayLibrary.Array_Set` (`self.isPointValid`) Index)
            (`self.InvalidatePoint` Index Start)
            (break)))
        (else
          (`KismetArrayLibrary.Array_Set` (`self.isPointValid`) Index false true)
          (`self.InvalidatePoint` Index Start)
          (break))))
    (else
      (`KismetArrayLibrary.Array_Set` (`self.isPointValid`) Index false true)))
  (`self.InvalidatePoint` Index Start))

(event `CheckForGround`
  (bind (_returnvalue_x _returnvalue_y _returnvalue_z) (`KismetMathLibrary.BreakVector` (`self.K2_GetActorLocation`)))
  (bind _returnvalue (* (`self.gridCellSize`) 0.5))
  ;[1 1 1] For each point, check if it's on the ground then adjust location
  (for (_array_element _array_index) (`self.gridPointsArray`)
    (`self.CheckFloor` _array_element _array_element (`KismetMathLibrary.MakeVector` _returnvalue _returnvalue _returnvalue) _array_index))
  (for _array_element_2 (`self.gridPointsToRemove`)
    (`KismetArrayLibrary.Array_RemoveItem` (`self.gridPointsArray`) _array_element_2))
  (`KismetArrayLibrary.Array_Clear` (`self.gridPointsToRemove`))
  (for _array_element_3 (`self.gridPointsToAdjust`)
    (`KismetArrayLibrary.Array_Set` (`self.gridPointsArray`) (`KismetArrayLibrary.Array_Find` (`self.gridPointsArray`) (`KismetMathLibrary.MakeVector` (.x _array_element_3) (.y _array_element_3) _returnvalue_z)) _array_element_3 true))
  (`KismetArrayLibrary.Array_Clear` (`self.gridPointsToAdjust`)))

(fn `GetNearestPoint`
  (params (HitPoint :type "Vector Structure"))
  (returns (NearestLocation :type "Vector Structure (by ref)"))
  (locals (ClosestIndex :type Integer :default 0) (ClosestDistance :type "Float (double-precision)" :default 0.0))
  (if (`KismetArrayLibrary.Array_IsNotEmpty` (`self.gridPointsArray`))
    (for (_array_element _array_index) (`self.gridPointsArray`)
      (if (== _array_index 0)
        (bind _returnvalue (`KismetMathLibrary.Vector_DistanceSquared` _array_element HitPoint))
        (set `local.ClosestDistance` _returnvalue)
        (set `local.ClosestIndex` 0)
        (elif (< _returnvalue (`local.ClosestDistance`))
          (set `local.ClosestDistance` _returnvalue)
          (set `local.ClosestIndex` _array_index))))
    (return (`|GetArrayItem` (`self.gridPointsArray`) (`local.ClosestIndex`)))
    (else
      (return (`|GetArrayItem` (`self.gridPointsArray`) (`local.ClosestIndex`))))))

(fn `UserConstructionScript`
  (`BoxComponent.SetBoxExtent` (`self.Box`) (`self.BoxSize`) true))