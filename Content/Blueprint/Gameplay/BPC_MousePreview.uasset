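; Player component that positions BP_Player's WidgetMouse in the world as a preview cursor for the mouse or grabbed furniture.
; A fast looping timer places the widget at the deprojected mouse position, or on the grabbed item.
; After a furniture change, a short delay starts constant-speed interpolation, which switches to snapping once the widget is close.
; MoveMouse nudges the screen cursor from input when nothing is grabbed and runs a debug-drawn line trace.
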(event `Tick`
  (bind _grabbeditem (`self.grabbedItem`))
  (bind _mouseref (`self.mouseRef`))
  (bind _returnvalue (`SceneComponent.K2_GetComponentLocation` (`Actor.RootComponent` _grabbeditem)))
  (if (`KismetSystemLibrary.IsValid` _grabbeditem)
    (`SceneComponent.K2_SetWorldLocation` _mouseref (`KismetMathLibrary.SelectVector` (`KismetMathLibrary.VInterpTo_Constant` (`SceneComponent.K2_GetComponentLocation` (`self.mouseRef`)) _returnvalue 0.001 500.0) _returnvalue (`self.lerpSpeed`)) false false)
    (else
      (`SceneComponent.K2_SetWorldLocation` _mouseref (`PlayerController.DeprojectMousePositionToWorld` (`GameplayStatics.GetPlayerController` 0)) false false))))

(event `self.ReceiveBeginPlay`
  (bind _asbp_player (cast `/Game/Blueprint/Character/BP_Player` (`self.GetOwner`)))
  (set `self.mouseRef` (`/Game/Blueprint/Character/BP_Player.Widget_Mouse` _asbp_player))
  (add `/Game/Blueprint/Character/BP_Player.FurnitureChange` _asbp_player (delegate `FurnitureChange`))
  (`KismetSystemLibrary.K2_SetTimerDelegate` (delegate `Tick`) 0.001 true true))

(event `FurnitureChange`
  (params (furniture :type "/Game/Blueprint/Gameplay/BP_Furniture Object Reference"))
  (`/Engine/EditorBlueprintResources/StandardMacros.IsValid` furniture
    (:`Is Valid`
      (`KismetSystemLibrary.Delay` 0.3)
      (set `self.grabbedItem` furniture)
      (set `self.lerpSpeed` true)
      (`KismetSystemLibrary.Delay` 0.1 :!label _label)
      (if (< (`KismetMathLibrary.Vector_DistanceSquared` (`SceneComponent.K2_GetComponentLocation` (`self.mouseRef`)) (`SceneComponent.K2_GetComponentLocation` (`Actor.RootComponent` (`self.grabbedItem`)))) 500000.0)
        (set `self.lerpSpeed` false)
        (else
          (goto _label))))
    (:`Is Not Valid`
      (set `self.grabbedItem` furniture))))

(event `MoveMouse`
  (params (actionValue :type "Vector2D Structure"))
  (bind _returnvalue (`GameplayStatics.GetPlayerController` 0))
  (bind (_locationx _locationy) (`PlayerController.GetMousePosition` _returnvalue))
  (bind _worldlocation (`PlayerController.DeprojectMousePositionToWorld` _returnvalue))
  (bind (_returnvalue_x _returnvalue_y) (`KismetMathLibrary.BreakVector2D` (+ (* actionValue (10.0 -10.0)) (`KismetMathLibrary.MakeVector2D` _locationx _locationy))))
  ;[0 0 0] ClampMouseMovement
  (`/Engine/EditorBlueprintResources/StandardMacros.IsValid` (`self.grabbedItem`)
    (:`Is Not Valid`
      (`PlayerController.SetMouseLocation` _returnvalue (`KismetMathLibrary.FTrunc` _returnvalue_x) (`KismetMathLibrary.FTrunc` _returnvalue_y))
      (`KismetSystemLibrary.LineTraceSingle` :`Start` _worldlocation :`End` (+ _worldlocation (* (`KismetMathLibrary.GetForwardVector` (`KismetMathLibrary.FindLookAtRotation` (`PlayerCameraManager.GetCameraLocation` (`GameplayStatics.GetPlayerCameraManager` 0)) (`SceneComponent.K2_GetComponentLocation` (`self.mouseRef`)))) 10000.0)) :`TraceChannel` "TraceTypeQuery1" :`DrawDebugType` "ForDuration"))))