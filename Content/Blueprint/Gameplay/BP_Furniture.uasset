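; Grid-snapped furniture actor that the player spawns, moves, rotates in 45-degree steps, places, lifts to modify, or deletes.
; Timelines animate each action, tuned by a furniture data asset.
; A tap steps toward the next grid point, while a hold moves with acceleration relative to the pawn and snaps on release.
; A looping box trace colors the shadow decal green or red, and invalid placement triggers a rotation shake.
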(event `self.ReceiveBeginPlay`
  (bind _furnituredataasset (`self.furnitureDataAsset`))
  (bind _snaptogridlerpspeed (`/Game/Data/DataAsset/BP/BP_FurnitureDA.snapToGridLerpSpeed` (`self.furnitureDataAsset`)))
  (bind _placelerpspeed (`/Game/Data/DataAsset/BP/BP_FurnitureDA.placeLerpSpeed` (`self.furnitureDataAsset`)))
  (bind (_output_previewimage _output_mesh) (break `/Game/Data/Struct/S_Furniture` (`|GetArrayItem` (`.Varianttype_21_E2AE205547457FD2E6B3DFB241F258D6` (break `/Game/Data/Struct/S_FurnitureShop` (`self.furnitureData`))) (`self.variantIndex`))))
  ;[0 0.1469 1] Begin play
  (bind _returnvalue (`GameplayStatics.GetActorOfClass` "/Game/Blueprint/Gameplay/BP_GridManager.BP_GridManager_C"))
  (bind _output_get (set `self.gridManagerRef` _returnvalue))
  (`|ExecutionSequence`
    (:`then_0`
      (`self.K2_SetActorRotation` (`KismetMathLibrary.MakeRotator` 0.0))
      (`TimelineComponent.SetPlayRate` (`self.StopLerpTL`) _snaptogridlerpspeed)
      (`TimelineComponent.SetPlayRate` (`self.MoveLerpTL`) _snaptogridlerpspeed)
      (`StaticMeshComponent.SetStaticMesh` (`self.baseMesh`) _output_mesh)
      (`TimelineComponent.SetPlayRate` (`self.DeleteLerpTL`) (`/Game/Data/DataAsset/BP/BP_FurnitureDA.destroyLerpSpeed` (`self.furnitureDataAsset`)))
      (`TimelineComponent.SetPlayRate` (`self.SpawnLerpTL`) (`/Game/Data/DataAsset/BP/BP_FurnitureDA.spawnLerpSpeed` (`self.furnitureDataAsset`)))
      (`TimelineComponent.SetPlayRate` (`self.PlaceObjectTL`) _placelerpspeed)
      (`TimelineComponent.SetPlayRate` (`self.ModifyLerpTL`) _placelerpspeed)
      (`TimelineComponent.SetPlayRate` (`self.Timeline`) (`/Game/Data/DataAsset/BP/BP_FurnitureDA.errorLerpSpeed` (`self.furnitureDataAsset`)))
      (`self.SetActorScale3D` (1.0 1.0 1.0))
      (set `self.startActorScale` (`self.GetActorScale3D`))
      (set `self.startActorRotation` (`self.K2_GetActorRotation`)))
    (:`then_1`
      (bind _nearestlocation (`/Game/Blueprint/Gameplay/BP_GridManager.GetNearestPoint` _output_get (`self.K2_GetActorLocation`)))
      (bind (_direction _alpha) (`Timeline|SpawnLerpTL` :!via `PlayFromStart`)
        (:`Update`
          (bind (_vectorwithoutz_x _vectorwithoutz_y) (`KismetMathLibrary.BreakVector` (`self.Remove Z` _nearestlocation true)))
          (`self.K2_SetActorLocation` (`KismetMathLibrary.MakeVector` _vectorwithoutz_x _vectorwithoutz_y (`KismetMathLibrary.Lerp` (`/Game/Data/DataAsset/BP/BP_FurnitureDA.spawnAnimStartZ` _furnituredataasset) (`/Game/Data/DataAsset/BP/BP_FurnitureDA.spawnAnimEndZ` _furnituredataasset) _alpha)))
          (`self.SetActorScale3D` (`KismetMathLibrary.VLerp` (1e-06 1e-06 1e-06) (1.0 1.0 1.0) (`KismetMathLibrary.FClamp` _alpha 0.0 2.0)))
          (bind _returnvalue_2 (`KismetSystemLibrary.K2_SetTimerDelegate` (delegate `CanBePlaceCheck`) 0.01 true true))
          (set `self.checkPlacementRef` _returnvalue_2))))))

(event `CanBePlaceCheck`
  (bind (_returnvalue_x _returnvalue_y) (`KismetMathLibrary.BreakVector` (`self.K2_GetActorLocation`)))
  (bind (_returnvalue_x_2 _returnvalue_y_2 _returnvalue_z) (`KismetMathLibrary.BreakVector` (`self.K2_GetActorLocation` (`self.gridManagerRef`))))
  (bind _returnvalue (`KismetMathLibrary.MakeVector` _returnvalue_x _returnvalue_y _returnvalue_z))
  ;[1 1 1] Check if it can be placed
  (bind _outhits (`KismetSystemLibrary.BoxTraceMultiForObjects` :`Start` _returnvalue :`End` _returnvalue :`HalfSize` (`BoxComponent.BoxExtent` (`self.Box`)) :`Orientation` (`self.K2_GetActorRotation`) :`ObjectTypes` (`|MakeArray` "ObjectTypeQuery7" "ObjectTypeQuery8" :!type "EObjectTypeQuery Enum") :`DrawDebugType` "ForOneFrame"))
  (if (`KismetArrayLibrary.Array_IsNotEmpty` _outhits)
    (set `self.CanBePlaced` false)
    (else
      (set `self.CanBePlaced` true)))
  (`self.ChangeShadowColor` (`self.CanBePlaced`)))

(event `MoveFurniture`
  (params (actionValue :type "Vector2D Structure") (triggeredTime :type "Float (double-precision)"))
  (bind (_returnvalue_x _returnvalue_y _returnvalue_z) (`KismetMathLibrary.BreakVector` (`self.K2_GetActorLocation`)))
  (bind _returnvalue (`GameplayStatics.GetPlayerPawn` 0))
  (bind (_returnvalue_x_2 _returnvalue_y_2 _returnvalue_z_2) (`KismetMathLibrary.BreakVector` (`self.K2_GetActorLocation`)))
  (bind _returnvalue_2 (`GameplayStatics.GetPlayerPawn` 0))
  (bind _furnituredataasset (`self.furnitureDataAsset`))
  (bind _gridcellsize (`/Game/Blueprint/Gameplay/BP_GridManager.gridCellSize` (`self.gridManagerRef`)))
  (bind (_x _y) (`KismetMathLibrary.BreakVector2D` (`KismetMathLibrary.Normal2D` (`self.Direction`))))
  (bind _returnvalue_3 (* (`/Game/Blueprint/Gameplay/BP_GridManager.gridCellSize` (`self.gridManagerRef`)) (`GameplayStatics.GetWorldDeltaSeconds`) (`self.speed`)))
  (bind (_returnvalue_x_3 _returnvalue_y_3) (`KismetMathLibrary.BreakVector` (+ (* (`self.GetActorForwardVector` _returnvalue_2) (`KismetMathLibrary.Round` _x) _gridcellsize 1.3) (* (`self.GetActorRightVector` _returnvalue_2) (`KismetMathLibrary.Round` _y) _gridcellsize 1.3))))
  ;[1 1 1] Move the furniture
  (if (< (`self.speed`) (`/Game/Data/DataAsset/BP/BP_FurnitureDA.maxMoveSpeed` _furnituredataasset))
    (set `self.speed` (+ (`self.speed`) (* (`GameplayStatics.GetWorldDeltaSeconds`) (`/Game/Data/DataAsset/BP/BP_FurnitureDA.acceleration` _furnituredataasset) (* triggeredTime 0.95)))))
  (if (>= triggeredTime (`/Game/Data/DataAsset/BP/BP_FurnitureDA.holdTimeTreshold` (`self.furnitureDataAsset`)))
    (`TimelineComponent.Stop` (`self.MoveLerpTL`))
    (`self.ResetMovingNextLoc`)
    (`self.ResetMoveToNextLocation`)
    (else
      (set `self.Direction` (`KismetMathLibrary.Normal2D` actionValue))
      (`|ExecutionSequence`
        (:`then_0`
          (`/Engine/EditorBlueprintResources/StandardMacros.DoOnce` false :!label _label
            (:`Completed`
              (set `self.MoveNextLocation` (`KismetMathLibrary.MakeVector` (+ _returnvalue_x_3 _returnvalue_x_2) (+ _returnvalue_y_3 _returnvalue_y_2) _returnvalue_z_2)))))
        (:`then_1`
          _))))
  (if (!= actionValue (0.0 0.0))
    (bind _output_get (set `self.Direction` (`KismetMathLibrary.Normal2D` actionValue))))
  (bind (_returnvalue_x_4 _returnvalue_y_4) (`KismetMathLibrary.BreakVector` (+ (* (`self.GetActorForwardVector` _returnvalue) (`KismetMathLibrary.BreakVector2D` _output_get) _returnvalue_3) (* (`self.GetActorRightVector` _returnvalue) (`.Y` (`KismetMathLibrary.BreakVector2D` _output_get)) _returnvalue_3))))
  (`self.K2_SetActorLocation` (`KismetMathLibrary.MakeVector` (+ _returnvalue_x_4 _returnvalue_x) (+ _returnvalue_y_4 _returnvalue_y) _returnvalue_z) true)
  (`TimelineComponent.Stop` (`self.StopLerpTL`)))

(event `ResetMoveToNextLocation`
  ;[1 1 1] Move the furniture
  (goto _label :!via `Reset`))

(event `DeleteFurniture`
  ;[1 1 1] Destroy furniture
  (set `self.startActorScale` (`self.GetActorScale3D`))
  (bind (_direction _alpha) (`Timeline|DeleteLerpTL` :!via `PlayFromStart`)
    (:`Update`
      (`self.SetActorScale3D` (`KismetMathLibrary.VLerp` (`self.startActorScale`) (0.0 0.0 0.0) _alpha)))
    (:`Finished`
      (`self.K2_DestroyActor`))))

(event `StopMovingFurniture`
  (params (triggeredTime :type "Float (double-precision)"))
  (bind _returnvalue (`self.K2_GetActorLocation`))
  ;[1 1 1] Stop the furniture moving and lerp it to the nearest point
  (set `self.speed` 0.0)
  (if (>= triggeredTime (`/Game/Data/DataAsset/BP/BP_FurnitureDA.holdTimeTreshold` (`self.furnitureDataAsset`)))
    (if (not (`self.IsAlreadyMoving`))
      (bind _nearestlocation (`/Game/Blueprint/Gameplay/BP_GridManager.GetNearestPoint` (`self.gridManagerRef`) _returnvalue))
      (bind _output_get (set `self.moveStartLocation` _returnvalue))
      (bind (_direction _alpha) (`Timeline|StopLerpTL` :!via `PlayFromStart`)
        (:`Update`
          (`self.K2_SetActorLocation` (`KismetMathLibrary.VLerp` _output_get (`self.Remove Z` _nearestlocation true) _alpha) true))))
    (else
      (`/Engine/EditorBlueprintResources/StandardMacros.DoOnce` false :!label _label_2
        (:`Completed`
          (bind _nearestlocation_2 (`/Game/Blueprint/Gameplay/BP_GridManager.GetNearestPoint` (`self.gridManagerRef`) (`self.MoveNextLocation`)))
          (set `self.IsAlreadyMoving` true)
          (bind _output_get_2 (set `self.moveStartLocation` (`self.K2_GetActorLocation`)))
          (bind (_direction_2 _alpha_2) (`Timeline|MoveLerpTL` :!via `PlayFromStart`)
            (:`Update`
              (`self.K2_SetActorLocation` (`KismetMathLibrary.VLerp` _output_get_2 (`self.Remove Z` _nearestlocation_2 true) _alpha_2) true))
            (:`Finished`
              (`self.ResetMovingNextLoc`)
              (`self.ResetMoveToNextLocation`))))))))

(event `CantPlaceFurniture`
  (bind (_returnvalue_roll _returnvalue_pitch _returnvalue_yaw) (`KismetMathLibrary.BreakRotator` (`self.K2_GetActorRotation`)))
  (bind (_errorrotationamplitude_x _errorrotationamplitude_y _errorrotationamplitude_z) (`KismetMathLibrary.BreakVector` (`/Game/Data/DataAsset/BP/BP_FurnitureDA.errorRotationAmplitude` (`self.furnitureDataAsset`))))
  ;[1 1 1] Can't Place Furniture
  (set `self.isShaking` true)
  (bind (_direction _endlerpalpha) (`Timeline|Timeline` :!via `PlayFromStart`)
    (:`Update`
      (if (not (`self.isShaking`))
        (`self.K2_SetActorRotation` (`KismetMathLibrary.RLerp` (`self.K2_GetActorRotation`) (`self.startActorRotation`) _endlerpalpha))
        (else
          (`self.K2_SetActorRotation` (`KismetMathLibrary.MakeRotator` (+ _returnvalue_roll (`KismetMathLibrary.RandomFloatInRange` (* _errorrotationamplitude_x -1.0) _errorrotationamplitude_x)) (+ _returnvalue_pitch (`KismetMathLibrary.RandomFloatInRange` (* _errorrotationamplitude_y -1.0) _errorrotationamplitude_y)) (+ _returnvalue_yaw (`KismetMathLibrary.RandomFloatInRange` (* _errorrotationamplitude_z -1.0) _errorrotationamplitude_z)))))))
    (:`FinishedBis`
      (set `self.isShaking` false))))

(event `ResetMovingNextLoc`
  ;[1 1 1] Stop the furniture moving and lerp it to the nearest point
  (set `self.IsAlreadyMoving` false)
  (goto _label_2 :!via `Reset`))

(event `RotateFurniture`
  (params (direction :type Integer))
  (bind (_returnvalue_roll _returnvalue_pitch _returnvalue_yaw) (`KismetMathLibrary.BreakRotator` (`self.K2_GetActorRotation`)))
  ;[1 1 1] Rotate object
  (if (== direction (`self.previousDirection`))
    (`/Engine/EditorBlueprintResources/StandardMacros.DoOnce` false :!label _label_3
      (:`Completed`
        _)))
  (`self.SetRotationIndex` direction)
  (set `self.actualRot` _returnvalue_yaw)
  (`|ExecutionSequence`
    (:`then_0`
      (bind (_direction _alpha) (`Timeline|RotationLerpTL` :!via `PlayFromStart`)
        (:`Update`
          (`self.K2_SetActorRotation` (`KismetMathLibrary.RLerp` (`KismetMathLibrary.MakeRotator` 0.0 0.0 (`self.actualRot`)) (`KismetMathLibrary.MakeRotator` 0.0 0.0 (select `int` (`self.newRotIndex`) :`0` 0.0 :`1` 45.0 :`2` 90.0 :`3` 135.0 :`4` 180.0 :`5` 225.0 :`6` 270.0 :`7` 315.0)) _alpha true) true))
        (:`Finished`
          (set `self.startActorRotation` (`self.K2_GetActorRotation`)))))
    (:`then_1`
      (`KismetSystemLibrary.RetriggerableDelay` 0.2)
      (`self.ResetRot`))))

(event `ResetRot`
  ;[1 1 1] Rotate object
  (goto _label_3 :!via `Reset`))

(event `PlaceFurniture`
  ;[1 1 1] Place Furniture
  (if (and (`|EnumInequality` (`self.state`) "NewEnumerator1") (`self.CanBePlaced`))
    (`TimelineComponent.Stop` (`self.ModifyLerpTL`))
    (`TimelineComponent.Stop` (`self.Timeline`))
    (`/Engine/EditorBlueprintResources/StandardMacros.DoOnce` false :!label _label_4
      (:`Completed`
        (bind _nearestlocation (`/Game/Blueprint/Gameplay/BP_GridManager.GetNearestPoint` (`self.gridManagerRef`) (`self.K2_GetActorLocation`)))
        (bind (_direction _alphapos _alphascale) (`Timeline|PlaceObjectTL` :!via `PlayFromStart`)
          (:`Update`
            (`self.K2_SetActorLocation` (`KismetMathLibrary.VLerp` (`KismetMathLibrary.MakeVector` (.x (`self.K2_GetActorLocation`)) (.y (`self.K2_GetActorLocation`)) (.z (`self.K2_GetActorLocation`))) (`KismetMathLibrary.MakeVector` (.x _nearestlocation) (.y _nearestlocation) (.z _nearestlocation)) _alphapos))
            (`self.SetActorScale3D` (`KismetMathLibrary.VLerp` (0.0 0.0 0.0) (`self.startActorScale`) (`KismetMathLibrary.FClamp` _alphascale 0.0 2.0))))
          (:`Finished`
            (`ActorComponent.SetActive` (`self.Shadow`) false false)
            (`ActorComponent.SetActive` (`self.SceneCaptureComponent2D`) false false)
            (message `/Game/Blueprint/_BPI/BPI_Player.SetFurnitureRef` (`GameplayStatics.GetPlayerPawn` 0) null)
            (`self.ResetPlaceTimeline`)
            (`KismetSystemLibrary.K2_PauseTimerHandle` (`self.checkPlacementRef`))
            (`self.K2_SetActorRotation` (`self.startActorRotation`))
            (set `self.state` "NewEnumerator1"))
          (:`CameraShake`
            (if (`KismetArrayLibrary.Array_IsNotEmpty` (`PrimitiveComponent.GetOverlappingActors` (`self.Box`) "BP_Furniture_C"))
              (`TimelineComponent.Stop` (`self.PlaceObjectTL`))
              (`self.CantPlaceFurniture`)
              (`self.ModifyFurniture`)
              (else
                (`PlayerController.ClientStartCameraShake` :`self` (`GameplayStatics.GetPlayerController` 0) :`Shake` "/Game/Data/Shakes/CS_Placement.CS_Placement_C")))))))
    (else
      (`self.CantPlaceFurniture`))))

(event `ResetPlaceTimeline`
  ;[1 1 1] Place Furniture
  (goto _label_4 :!via `Reset`))

(event `ModifyFurniture`
  (bind _returnvalue (`self.K2_GetActorLocation`))
  ;[1 1 1] Modify Furniture
  (if (`|EnumInequality` (`self.state`) "NewEnumerator0")
    (bind (_direction _localpha _sizealpha) (`Timeline|ModifyLerpTL` :!via `PlayFromStart`)
      (:`Update`
        (`self.K2_SetActorLocation` (`KismetMathLibrary.VLerp` _returnvalue (`KismetMathLibrary.MakeVector` (.x _returnvalue) (.y _returnvalue) (`/Game/Data/DataAsset/BP/BP_FurnitureDA.spawnAnimEndZ` (`self.furnitureDataAsset`))) _localpha))
        (`self.SetActorScale3D` (`KismetMathLibrary.VLerp` (`self.GetActorScale3D`) (`self.startActorScale`) (`KismetMathLibrary.FClamp` _sizealpha 0.0 2.0))))
      (:`FinishedBis`
        (set `self.state` "NewEnumerator0")
        (`ActorComponent.SetActive` (`self.Shadow`) true false)
        (`ActorComponent.SetActive` (`self.SceneCaptureComponent2D`) true false)
        (`KismetSystemLibrary.K2_UnPauseTimerHandle` (`self.checkPlacementRef`))))))

(fn `ChangeShadowColor`
  (params (canBePlaced :type Boolean))
  (bind _shadow (`self.Shadow`))
  (if canBePlaced
    (`DecalComponent.SetDecalMaterial` _shadow "/Game/Blueprint/ColoredShadows/MI_ShadowGreen.MI_ShadowGreen")
    (else
      (`DecalComponent.SetDecalMaterial` _shadow "/Game/Blueprint/ColoredShadows/MI_ShadowRed.MI_ShadowRed"))))

(fn `OnRep_CanBePlaced`)

(fn `Remove Z`
  (params (Vector :type "Vector Structure") (UseActorZ :type Boolean))
  (returns (vectorWithoutZ :type "Vector Structure"))
  (bind (_returnvalue_x _returnvalue_y _returnvalue_z) (`KismetMathLibrary.BreakVector` (`self.K2_GetActorLocation`)))
  (if UseActorZ
    (return (`KismetMathLibrary.MakeVector` Vector_X Vector_Y _returnvalue_z))
    (else
      (return (`KismetMathLibrary.MakeVector` Vector_X Vector_Y)))))

(fn `ResizeBox`
  (bind (_origin _boxextent) (`KismetSystemLibrary.GetComponentBounds` (`self.baseMesh`)))
  (bind (_returnvalue_x _returnvalue_y _returnvalue_z) (`KismetMathLibrary.BreakVector` (- _boxextent (`/Game/Data/DataAsset/BP/BP_FurnitureDA.boxCollisionOffset` (`self.furnitureDataAsset`)))))
  (`BoxComponent.SetBoxExtent` (`self.Box`) (`KismetMathLibrary.MakeVector` _returnvalue_x _returnvalue_y _returnvalue_z) true)
  (`SceneComponent.K2_SetWorldLocation` (`self.Box`) _origin false false))

(fn `UserConstructionScript`
  (bind (_output_previewimage _output_mesh) (break `/Game/Data/Struct/S_Furniture` (`|GetArrayItem` (`.Varianttype_21_E2AE205547457FD2E6B3DFB241F258D6` (break `/Game/Data/Struct/S_FurnitureShop` (`self.furnitureData`))) (`self.variantIndex`))))
  (`SceneCaptureComponent.ShowOnlyComponent` (`self.SceneCaptureComponent2D`) (`self.baseMesh`))
  (`StaticMeshComponent.SetStaticMesh` (`self.baseMesh`) _output_mesh)
  (`self.ChangeShadowColor` (`self.CanBePlaced`))
  (`self.ResizeBox`))