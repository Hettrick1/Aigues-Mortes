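; BP_Itch is a showcase camera rig that rotates while the tower cycles through set-dress scenes.
; Construction frames the spring-arm camera using player and Itch data assets.
; A looping timer passes each configured scene to BP_TowerSetDress.
; A duration-scaled timeline drives optionally eased yaw rotation and writes DissolvePos, initially placed at the camera, into MPC_General's PlayerPos, standing in for the player.
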(event `self.ReceiveBeginPlay`
  (bind _itchdataasset (`self.itchDataAsset`))
  (bind (_returnvalue_x _returnvalue_y _returnvalue_z) (`KismetMathLibrary.BreakVector` (`SceneComponent.K2_GetComponentLocation` (`self.dissolvePos`))))
  (bind _returnvalue (`GameplayStatics.GetActorOfClass` "/Game/Blueprint/Tower/BP_TowerSetDress.BP_TowerSetDress_C"))
  (set `self.setDressRef` _returnvalue)
  (`SceneComponent.K2_SetWorldLocation` (`self.dissolvePos`) (`SceneComponent.K2_GetComponentLocation` (`self.Camera`)) false false)
  (`KismetSystemLibrary.K2_SetTimerDelegate` (delegate `changeSetDress`) (`/Game/Data/DataAsset/BP/BP_ItchIoDA.delayBetwenScenes` (`self.itchDataAsset`)) true true)
  (`self.changeSetDress`)
  (`TimelineComponent.SetPlayRate` (`self.lerpDown`) (/ 1.0 (`/Game/Data/DataAsset/BP/BP_ItchIoDA.duration` (`self.itchDataAsset`))))
  (bind (_direction _lerp _lerplinear) (`Timeline|lerpDown` :!via `PlayFromStart`)
    (:`Update`
      (`self.K2_AddActorWorldRotation` (`KismetMathLibrary.MakeRotator` 0.0 0.0 (`KismetMathLibrary.Lerp` 0.0 (`/Game/Data/DataAsset/BP/BP_ItchIoDA.rotationSpeed` _itchdataasset) (`KismetMathLibrary.SelectFloat` _lerp _lerplinear (`/Game/Data/DataAsset/BP/BP_ItchIoDA.easeInOut` _itchdataasset)))))
      (`KismetMaterialLibrary.SetVectorParameterValue` "/Game/Art/CoreMat/MPC/MPC_General.MPC_General" "PlayerPos" (make `LinearColor` _returnvalue_x _returnvalue_y _returnvalue_z 1.0)))))

(event `changeSetDress`
  (`/Game/Blueprint/Tower/BP_TowerSetDress.SetWall` (`self.setDressRef`) (make `/Game/Data/Struct/S_Walls` "" "" "" "" "" "" null (`|GetArrayItem` (`/Game/Data/DataAsset/BP/BP_ItchIoDA.scenes` (`self.itchDataAsset`)) (`self.sceneIndex`))))
  (set `self.sceneIndex` (`KismetMathLibrary.SelectInt` 0 (+ (`self.sceneIndex`) 1) (== (`self.sceneIndex`) (`KismetArrayLibrary.Array_LastIndex` (`/Game/Data/DataAsset/BP/BP_ItchIoDA.scenes` (`self.itchDataAsset`))))))
  (if (`KismetArrayLibrary.Array_IsEmpty` (`/Game/Data/DataAsset/BP/BP_ItchIoDA.scenes` (`self.itchDataAsset`)))
    (`KismetSystemLibrary.PrintString` "No set dress to display")))

(fn `UserConstructionScript`
  (bind _playerdataasset (`self.playerDataAsset`))
  (`CameraComponent.SetFieldOfView` (`self.Camera`) (`/Game/Data/DataAsset/BP/BP_PlayerDA.baseFOV` _playerdataasset))
  (`SceneComponent.K2_SetRelativeRotation` (`self.Camera`) (`KismetMathLibrary.MakeRotator` 0.0 (* (`/Game/Data/DataAsset/BP/BP_PlayerDA.cameraAngle` _playerdataasset) -1.0)) false false)
  (`SceneComponent.K2_SetRelativeRotation` (`self.SpringArm`) (`KismetMathLibrary.MakeRotator` 0.0 (* (`/Game/Data/DataAsset/BP/BP_PlayerDA.springArmAngle` _playerdataasset) -1.0)) false false)
  (set `SpringArmComponent.TargetArmLength` (`/Game/Data/DataAsset/BP/BP_ItchIoDA.camDistance` (`self.itchDataAsset`)) (`self.SpringArm`)))