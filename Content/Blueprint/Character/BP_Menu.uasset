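; BP_Menu is a menu Blueprint that sets up CineCamera focus on the preview item, with an optional animated focus pull.
; On BeginPlay it measures the camera's distance to the BP_PreviewItem mesh and sets the timeline play rate from the data asset's FocusSpeed.
; A positive speed lerps manual focus from StartFocus toward that distance, tripling the lerped value; otherwise focus is set directly to the unscaled distance.
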(event `LerpFocus`
  ;[0 0 0] Load Data asset & PreviewMesh
  (if (> (`/Game/Data/DataAsset/BP/BP_WaitingScreenDA.focusSpeed` (`self.dataAssetRef`)) 0.0) :!label _label
    ;[0 0 0] Lerp Focus at desired speed
    (bind (_direction _alpha) (`Timeline|FocusTimeline` :!via `PlayFromStart`)
      (:`Update`
        (set `CineCameraComponent.FocusSettings` (make `CameraFocusSettings` "Manual" (* (`KismetMathLibrary.Lerp` (`/Game/Data/DataAsset/BP/BP_WaitingScreenDA.startFocus` (`self.dataAssetRef`)) (`self.cameraDistance`) _alpha) 3.0) (struct :`RelativeOffset` (0.0 0.0 0.0)) true) (`self.CineCamera`))))
    (else
      ;[0 0 0] No focus lerp
      (set `CineCameraComponent.FocusSettings` (make `CameraFocusSettings` "Manual" (`self.cameraDistance`)) (`self.CineCamera`)))))

(event `self.ReceiveBeginPlay`
  ;[0 0 0] Load Data asset & PreviewMesh
  (`TimelineComponent.SetPlayRate` (`self.FocusTimeline`) (`/Game/Data/DataAsset/BP/BP_WaitingScreenDA.focusSpeed` (`self.dataAssetRef`)))
  (bind _returnvalue (`GameplayStatics.GetActorOfClass` "/Game/Blueprint/Menu/BP_PreviewItem.BP_PreviewItem_C"))
  (set `self.cameraDistance` (`KismetMathLibrary.Vector_Distance` (`SceneComponent.K2_GetComponentLocation` (`/Game/Blueprint/Menu/BP_PreviewItem.SM_Item` _returnvalue)) (`SceneComponent.K2_GetComponentLocation` (`self.CineCamera`))))
  (goto _label))

(fn `UserConstructionScript`)