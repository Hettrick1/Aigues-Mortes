(event Custom|SetHudRef
  (params (hudRef :type WBP%20Quest%20Recap%20Object%20Reference))
  ;[0 0 0] Reference HUD
  (Variables|Default|SethudRef hudRef))

(event Custom|Tick
  (bind _dataasset (Variables|Default|GetdataAsset))
  (bind _dataasset_2 (Variables|Default|GetdataAsset))
  (bind _dataasset_3 (Variables|Default|GetdataAsset))
  (bind _camerarotation (Variables|Default|GetcameraRotation))
  (bind _playeroffset (Variables|Default|GetplayerOffset))
  (bind _zoomamount (Variables|Default|GetzoomAmount))
  (bind _dissolvepos (Variables|Default|GetdissolvePos))
  (bind _returnvalue (Transformation|GetWorldLocation _dissolvepos))
  (bind _camrotmaxangle (Variables|/Game/Data/DataAsset/BP/BP_PlayerDA.BP_PlayerDA_C|GetcamRotMaxAngle _dataasset_3))
  (bind _cameraangle (Variables|/Game/Data/DataAsset/BP/BP_PlayerDA.BP_PlayerDA_C|GetcameraAngle _dataasset))
  (bind _returnvalue_2 (* _camerarotation _camrotmaxangle))
  (bind (_x _y _z) (Math|Vector|BreakVector _returnvalue_2))
  ;[0 0 0] Add player offset when moving
  (Transformation|SetActorLocation (Math|Interpolation|VInterpTo (Transformation|GetActorLocation) (+ (Variables|Default|GetoriginLoc) (* (Transformation|GetActorRightVector) (.x _playeroffset)) (* (Transformation|GetActorForwardVector) (.y _playeroffset))) 0.005 (Variables|/Game/Data/DataAsset/BP/BP_PlayerDA.BP_PlayerDA_C|GetmovementSpeed (Variables|Default|GetdataAsset))) false false)
  (Variables|/Script/Engine.SpringArmComponent|SetTargetArmLength (Variables|Default|GetSpringArm) (Math|Interpolation|FInterpTo (Variables|/Script/Engine.SpringArmComponent|GetTargetArmLength (Variables|Default|GetSpringArm)) (Math|Float|SelectFloat (Variables|/Game/Data/DataAsset/BP/BP_PlayerDA.BP_PlayerDA_C|GetcamDistanceMin _dataasset_2) (Math|Float|SelectFloat (Variables|/Game/Data/DataAsset/BP/BP_PlayerDA.BP_PlayerDA_C|GetcamDistanceBase _dataasset_2) (Variables|/Game/Data/DataAsset/BP/BP_PlayerDA.BP_PlayerDA_C|GetcamDistanceMax _dataasset_2) (== _zoomamount 0.0)) (< _zoomamount 0.0)) 0.005 (Variables|/Game/Data/DataAsset/BP/BP_PlayerDA.BP_PlayerDA_C|GetcamZoom (Variables|Default|GetdataAsset))))
  (Transformation|SetRelativeRotation (Variables|Default|GetCineCamera) (Math|Interpolation|RInterpTo (Variables|/Script/Engine.SceneComponent|GetRelativeRotation (Variables|Default|GetCineCamera)) (Math|Rotator|MakeRotator 0.0 (* (Math|Float|Lerp _cameraangle (+ (Variables|/Game/Data/DataAsset/BP/BP_PlayerDA.BP_PlayerDA_C|GetcamZoomTilt _dataasset) _cameraangle) (Math|Float|Clamp(Float) (Variables|Default|GetzoomAmount) -1.0 0.0)) -1.0) 0.0) 0.005 (Variables|/Game/Data/DataAsset/BP/BP_PlayerDA.BP_PlayerDA_C|GetcamRotSpeed (Variables|Default|GetdataAsset))) false false)
  (Transformation|SetWorldRotation (Variables|Default|GetScene) (Math|Interpolation|RInterpTo (Transformation|GetWorldRotation (Variables|Default|GetScene)) (Math|Rotator|MakeRotator 0.0 (* _y -1.0) (+ _z (.yaw (Transformation|GetWorldRotation (Variables|Default|GetSpringArm))))) 0.005 (Variables|/Game/Data/DataAsset/BP/BP_PlayerDA.BP_PlayerDA_C|GetcamRotSpeed (Variables|Default|GetdataAsset))) false false)
  (Rendering|Material|SetVectorParameterValue "/Game/Art/CoreMat/MPC/MPC_General.MPC_General" "PlayerPos" (Utilities|Struct|MakeLinearColor (.x _returnvalue) (.y _returnvalue) (.z _returnvalue) 1.0) :!class /Script/Engine.KismetMaterialLibrary)
  (if (Variables|Default|GetisBuildMode)
    (|checkLocValid)))

(event Custom|ResetRot
  ;[0 0 0] RotateCharacter
  (Utilities|FlowControl|DoOnce false) ; enters at Reset
)

(event Custom|eventFurnitureChange
  (params (furniture :type BP%20Furniture%20Object%20Reference))
  (bind _returnvalue (Game|GetPlayerController 0))
  (bind _currentfurnitureref (Variables|Default|GetcurrentFurnitureRef))
  (bind _widget_mouse (Variables|Default|GetWidget_Mouse))
  (bind _returnvalue_2 (Transformation|GetWorldLocation _widget_mouse))
  (bind _screenposition (Class|GameplayStatics|ProjectWorldtoScreen _returnvalue _returnvalue_2 true))
  ;[0 0 0] Snap mouse to object
  (Utilities|IsValid furniture
    (:Is%20Valid
      (Default|SetHandWidget (Variables|Mouse|GetmouseWidgetRef) "NewEnumerator8")
      (Variables|Mouse|SetmouseLerping true)
      (Utilities|FlowControl|Delay (Utilities|Select :Index (Variables|/Game/Blueprint/Gameplay/BP_Furniture.BP_Furniture_C|Getstate furniture) :NewEnumerator0 0.3 :NewEnumerator1 0.0))
      (Variables|Mouse|SetpreviousMouseLoc (Transformation|GetWorldLocation (Variables|Default|GetWidget_Mouse)))
      (bind _lerp (Timeline|LerpMouse PlayFromStart)
        (:Update
          (Utilities|IsValid _currentfurnitureref
            (:Is%20Valid
              (Transformation|SetWorldLocation (Variables|Default|GetWidget_Mouse) (Math|Vector|Lerp(Vector) (Variables|Mouse|GetpreviousMouseLoc) (+ (Transformation|GetWorldLocation (Variables|/Game/Blueprint/Gameplay/BP_Furniture.BP_Furniture_C|GetbaseMesh _currentfurnitureref)) (Variables|/Game/Data/DataAsset/BP/BP_PlayerDA.BP_PlayerDA_C|GetmouseGrabbingOffset (Variables|Default|GetdataAsset))) _lerp) false false))
            (:Is%20Not%20Valid
              (Variables|Mouse|SetmouseLerping false :!label _label))))
        (:Finished
          (goto _label))))
    (:Is%20Not%20Valid
      (Class|PlayerController|SetMouseLocation _returnvalue (Math|Float|Truncate (.x _screenposition)) (Math|Float|Truncate (.y _screenposition)))
      (Variables|Mouse|SetmouseLerping false)
      (Default|SetHandWidget (Variables|Mouse|GetmouseWidgetRef) "NewEnumerator6"))))

(event EventMove
  (params (axis :type Vector%202D%20Structure))
  ;[0 0 0] Move player
  (if (Variables|Default|GetcanMove)
    (Variables|Default|SetplayerOffset (* (/ axis (Math|Vector2D|Vector2DLength axis)) (Variables|/Game/Data/DataAsset/BP/BP_PlayerDA.BP_PlayerDA_C|GetmovementMultiplyer (Variables|Default|GetdataAsset))))))

(event EventZoom
  (params (zoom :type Float%20%28double-precision%29))
  ;[0 0 0] Zoom
  (if (Variables|Default|GetcanMove)
    (bind _output_get (Variables|Default|SetzoomAmount (* zoom -1.0)))
    (Variables|Input|SetinverseRot (< _output_get 0.0))))

(event EventSetFurnitureRef
  (params (furnitureRef :type BP%20Furniture%20Object%20Reference))
  (bind _output_get (Variables|Default|SetcurrentFurnitureRef furnitureRef))
  (Utilities|IsValid (Utilities|SelectObject _output_get (Variables|Default|GetpreviousHitActor) (Utilities|IsValid _output_get))
    (:Is%20Valid
      (Class|BPIFurniture|ShowOutline(Message) (Utilities|SelectObject _output_get (Variables|Default|GetpreviousHitActor) (Utilities|IsValid _output_get)) false)
      (Variables|Default|SetpreviousHitActor 0))))

(event EventSetIsinBuildMode
  (params (isInBuildMode :type Boolean) (mouseIsFocus :type Boolean))
  (bind _returnvalue (Viewport|GetViewportSize))
  (bind _dataasset (Variables|Default|GetdataAsset))
  (bind _previoushitactor (Variables|Default|GetpreviousHitActor))
  (bind _returnvalue_2 (* _returnvalue 0.5))
  ;[0 0 0] Set is in build mode
  (if (Variables|Default|GetcanMove)
    (bind _output_get (Variables|Default|SetisBuildMode isInBuildMode))
    (Default|CallSetBuildMode _output_get)
    (Utilities|FlowControl|Sequence
      (:then_0
        (Development|SetHiddeninGame (Variables|Default|GetWidget_Mouse) (not _output_get) false))
      (:then_1
        (if _output_get
          (if mouseIsFocus
            _
            (else
              (Class|PlayerController|SetMouseLocation (Game|GetPlayerController 0) (Math|Float|Truncate (.x _returnvalue_2)) (Math|Float|Truncate (.y _returnvalue_2)))))
          (Variables|Default|SetcanMove false)
          (Variables|Default|SetzoomAmount 0.0)
          (bind _fovalpha (Timeline|ChangeModeTL PlayFromStart)
            (:Update
              (Camera|SetFieldOfView (Variables|Default|GetCineCamera) (Math|Float|Lerp (Variables|/Game/Data/DataAsset/BP/BP_PlayerDA.BP_PlayerDA_C|GetbaseFOV _dataasset) (Variables|/Game/Data/DataAsset/BP/BP_PlayerDA.BP_PlayerDA_C|GetbuildFOV _dataasset) _fovalpha)))
            (:Finished
              (Variables|Default|SetcanMove true)))
          (else
            (Utilities|IsValid _previoushitactor
              (:Is%20Valid
                (Class|BPIFurniture|ShowOutline(Message) _previoushitactor false))
              (:Is%20Not%20Valid
                _))
            (Utilities|IsValid (Variables|Default|GetcurrentFurnitureRef)
              (:Is%20Valid
                (Default|DeleteFurniture (Variables|Default|GetcurrentFurnitureRef))
                (Variables|Default|SetcurrentFurnitureRef 0)
                (Timeline|ChangeModeTL Reverse))
              (:Is%20Not%20Valid
                (Timeline|ChangeModeTL Reverse)))))))))

(event EventRotateCamera
  (params (direction :type Vector :default "0, 0, 0"))
  (if (Variables|Default|GetcanMove)
    (Variables|Default|SetcameraRotation direction)))

(event EventSpawnNewItem
  (params (struct :type S%20Furniture%20Shop%20Structure))
  ;[0 0 0] Spawn item
  (bind _returnvalue (Game|SpawnActorfromClass "/Game/Blueprint/Gameplay/BP_Furniture.BP_Furniture_C" (Math|Transform|MakeTransform "0.000000,0.000000,250.000000" "0, 0, 0" "1.000000,1.000000,1.000000") "AlwaysSpawn" "MultiplyWithRoot" 0 struct 0))
  (Variables|Default|SetcurrentFurnitureRef _returnvalue))

(event EventChangeVariant
  (bind (_start _end) (CallFunction|GetForwardfromMouse 1e+04))
  (bind _currentfurnitureref (Variables|Default|GetcurrentFurnitureRef))
  ;[0 0 0] If item in hand, change variant
  (Utilities|IsValid _currentfurnitureref
    (:Is%20Valid
      (Default|ChangeVariant _currentfurnitureref))
    (:Is%20Not%20Valid
      ;[0 0 0] Else, copy it
      (bind _outhit (Collision|LineTraceByChannel _start _end "TraceTypeQuery4" false 0 "None"))
      (if (Actor|ActorHasTag (.HitActor (Collision|BreakHitResult _outhit)) "Furniture")
        (bind _asbp_furniture (Utilities|Casting|CastToBP_Furniture (.HitActor (Collision|BreakHitResult _outhit))))
        (CallFunction|SpawnNewItem (Variables|/Game/Blueprint/Gameplay/BP_Furniture.BP_Furniture_C|GetfurnitureData _asbp_furniture))
        (Utilities|FlowControl|Delay 0.2)
        (Default|ChangeVariantIndex (Variables|Default|GetcurrentFurnitureRef) (Variables|/Game/Blueprint/Gameplay/BP_Furniture.BP_Furniture_C|GetvariantIndex _asbp_furniture))
        (Class|BPIFurniture|ShowOutline(Message) (Variables|Default|GetpreviousHitActor) false)
        (Variables|Default|SetpreviousHitActor 0)))))

(event EventEnableMovements
  (params (enable :type Boolean))
  ;[0 0 0] EnableMovements
  (Variables|Default|SetcanMove enable))

(event EventBeginPlay
  (bind _widget_mouse (Variables|Default|GetWidget_Mouse))
  ;[0 0 0] Save initla Location
  (Variables|Default|SetoriginLoc (Transformation|GetActorLocation))
  (Components|Timeline|SetPlayRate (Variables|Default|GetChangeModeTL) 4.0)
  (Transformation|SetWorldLocation (Variables|Default|GetdissolvePos) (Transformation|GetWorldLocation (Variables|Default|GetCineCamera)) false false)
  (Utilities|Time|SetTimerbyEvent (delegate Custom|Tick) 0.005 true true)
  ;[0 0 0] Snap mouse to object
  (if (Variables|Default|GetisBuildMode)
    (bind _aswbp_player_mouse (Utilities|Casting|CastToWBP_PlayerMouse (UserInterface|GetWidget (Variables|Default|GetWidget_Mouse))))
    (Variables|Mouse|SetmouseWidgetRef _aswbp_player_mouse)
    (EventDispatchers|BindEventtoFurnitureChange (delegate Custom|eventFurnitureChange))
    (else
      (bind _aswbp_player_mouse_2 (Utilities|Casting|CastToWBP_PlayerMouse (UserInterface|GetWidget _widget_mouse)))
      (Variables|Mouse|SetmouseWidgetRef _aswbp_player_mouse_2)
      (Development|SetHiddeninGame _widget_mouse true false)
      (EventDispatchers|BindEventtoFurnitureChange (delegate Custom|eventFurnitureChange)))))

(event EventRotate
  (params (direction :type Integer))
  ;[0 0 0] RotateCharacter
  (if (Variables|Default|GetcanMove)
    (if (== (Variables|Default|GetpreviousDirection) direction)
      (Utilities|FlowControl|DoOnce false
        (:Completed
          _)))
    (Utilities|SetRotationIndex (* direction (Math|Integer|SelectInt -1 1 (Variables|Input|GetinverseRot))))
    (Variables|Default|SetactualRot (.yaw (Transformation|GetActorRotation)))
    (Utilities|FlowControl|Sequence
      (:then_0
        (bind _alpha (Timeline|RotateCam PlayFromStart)
          (:Update
            (Transformation|SetActorRotation (Math|Rotator|Lerp(Rotator) (Math|Rotator|MakeRotator 0.0 0.0 (Variables|Default|GetactualRot)) (Math|Rotator|MakeRotator 0.0 0.0 (Utilities|Select :Index (Variables|Default|GetnewRotIndex) :Option%200 45.0 :Option%201 135.0 :Option%202 215.0 :Option%203 305.0)) _alpha true) true))
          (:Finished
            (CallFunction|MoveMouse))))
      (:then_1
        (Utilities|FlowControl|RetriggerableDelay (Variables|/Game/Data/DataAsset/BP/BP_PlayerDA.BP_PlayerDA_C|GetrotationDelay (Variables|Default|GetdataAsset)))
        (CallFunction|ResetRot)))))

(event EventMoveFurniture
  (params (direction :type Vector%202D%20Structure) (triggerTreshold :type Float%20%28double-precision%29))
  (bind _currentfurnitureref (Variables|Default|GetcurrentFurnitureRef))
  ;[0 0 0] Move / Stop moving furniture
  (Utilities|IsValid _currentfurnitureref
    (:Is%20Valid
      (Default|MoveFurniture _currentfurnitureref direction triggerTreshold))))

(event EventMoveMouse
  (params (actionValue :type Vector%202D%20Structure))
  (bind _returnvalue (Game|GetPlayerController 0))
  (bind (_start _end) (CallFunction|GetForwardfromMouse 1e+04))
  (bind _mousewidgetref (Variables|Mouse|GetmouseWidgetRef))
  (bind _dataasset (Variables|Default|GetdataAsset))
  (bind (_locationx _locationy) (Game|Player|GetMousePosition _returnvalue))
  (bind _mousesensitivity (Variables|/Game/Data/DataAsset/BP/BP_PlayerDA.BP_PlayerDA_C|GetmouseSensitivity _dataasset))
  (bind _returnvalue_2 (Math|Vector2D|MakeVector2D _locationx _locationy))
  (bind _returnvalue_3 (* _mousesensitivity -1.0))
  (bind _returnvalue_4 (* actionValue (Math|Vector2D|MakeVector2D _mousesensitivity _returnvalue_3)))
  (bind _returnvalue_5 (+ _returnvalue_4 _returnvalue_2))
  ;[0 0 0] ClampMouseMovement
  (if (Variables|Default|GetcanMove)
    (Utilities|IsValid (Variables|Default|GetcurrentFurnitureRef)
      (:Is%20Not%20Valid
        (Class|PlayerController|SetMouseLocation (Game|GetPlayerController 0) (Math|Float|Truncate (.x _returnvalue_5)) (Math|Float|Truncate (.y _returnvalue_5)))
        (bind (_outhit _returnvalue_6) (Collision|LineTraceByChannel _start _end "TraceTypeQuery4" false 0 "None"))
        ;[1 0 0] Code when hand is on item
        (if _returnvalue_6
          (if (Actor|ActorHasTag (.HitActor (Collision|BreakHitResult _outhit)) "Furniture")
            (Default|SetHandWidget _mousewidgetref "NewEnumerator7")
            (if (!= (Variables|Default|GetpreviousHitActor) (.HitActor (Collision|BreakHitResult _outhit)))
              (Utilities|IsValid (Variables|Default|GetpreviousHitActor)
                (:Is%20Valid
                  (Class|BPIFurniture|ShowOutline(Message) (Variables|Default|GetpreviousHitActor) false))
                (:Is%20Not%20Valid
                  _))
              (bind _output_get (Variables|Default|SetpreviousHitActor (.HitActor (Collision|BreakHitResult _outhit))))
              (Class|BPIFurniture|ShowOutline(Message) _output_get true))
            (else
              (if (not (Utilities|Enum|Equal(Enum) (Variables|/Game/Blueprint/UI/WBP_PlayerMouse.WBP_PlayerMouse_C|GethandState _mousewidgetref) "NewEnumerator9")) :!label _label
                (Default|SetHandWidget _mousewidgetref "NewEnumerator6")
                (Utilities|IsValid (Variables|Default|GetpreviousHitActor)
                  (:Is%20Valid
                    (Class|BPIFurniture|ShowOutline(Message) (Variables|Default|GetpreviousHitActor) false)
                    (Variables|Default|SetpreviousHitActor 0))))))
          (else
            (goto _label)))))))

(event EventRotateFurniture
  (params (direction :type Integer))
  (bind _currentfurnitureref (Variables|Default|GetcurrentFurnitureRef))
  ;[0 0 0] Move / Stop moving furniture
  (Utilities|IsValid _currentfurnitureref
    (:Is%20Valid
      (Default|RotateFurniture _currentfurnitureref direction))))

(event EventStopMovingFurniture
  (params (seconds :type Float%20%28double-precision%29))
  (bind _currentfurnitureref (Variables|Default|GetcurrentFurnitureRef))
  ;[0 0 0] Move / Stop moving furniture
  (Utilities|IsValid _currentfurnitureref
    (:Is%20Valid
      (Default|StopMovingFurniture _currentfurnitureref seconds))))

(event EventAcceptFurniture
  (bind (_start _end) (CallFunction|GetForwardfromMouse 1e+04))
  ;[0 0 0] Accept/Cancel furniture placement
  (Utilities|IsValid (Variables|Default|GetcurrentFurnitureRef)
    (:Is%20Valid
      (switch Utilities|FlowControl|Switch|SwitchonEnum_FurnitureState (Variables|/Game/Blueprint/Gameplay/BP_Furniture.BP_Furniture_C|Getstate (Variables|Default|GetcurrentFurnitureRef))
        (:NewEnumerator0
          (Default|PlaceFurniture (Variables|Default|GetcurrentFurnitureRef)))
        (:NewEnumerator1
          (Default|ModifyFurniture (Variables|Default|GetcurrentFurnitureRef)))))
    (:Is%20Not%20Valid
      (bind _outhit (Collision|LineTraceByChannel _start _end "TraceTypeQuery1" false 0 "None"))
      (bind _asbp_furniture (Utilities|Casting|CastToBP_Furniture (.HitActor (Collision|BreakHitResult _outhit))))
      (Variables|Default|SetcurrentFurnitureRef _asbp_furniture)
      (Default|ModifyFurniture _asbp_furniture))))

(event EventCancelFurniture
  ;[0 0 0] Accept/Cancel furniture placement
  (Utilities|IsValid (Variables|Default|GetcurrentFurnitureRef)
    (:Is%20Valid
      (Default|DeleteFurniture (Variables|Default|GetcurrentFurnitureRef))
      (Variables|Default|SetcurrentFurnitureRef 0))))

(event Input|KeyboardEvents|DebugKeyAdd
  (params (Key :type Key%20Structure :default "None") (ActionValue :type Input%20Action%20Value%20Structure))
  ;[0 0 0] Spawn item
  ;;[1 0.6921 0] DEBUG
  (:Pressed
    (bind _outrownames (DataTable|GetDataTableRowNames "/Game/Data/DataTable/DT_Furnitures.DT_Furnitures"))
    (Utilities|GetDataTableRow "/Game/Data/DataTable/DT_Furnitures.DT_Furnitures" (Utilities|Array|Get(acopy) _outrownames 20)
      (:then
        (bind _returnvalue (Game|SpawnActorfromClass "/Game/Blueprint/Gameplay/BP_Furniture.BP_Furniture_C" (Math|Transform|MakeTransform "0.000000,0.000000,250.000000" "0, 0, 0" "1.000000,1.000000,1.000000") "AlwaysSpawn" "MultiplyWithRoot" 0 (stale EventSpawnNewItem struct) 0))
        (Variables|Default|SetcurrentFurnitureRef _returnvalue)))))

(event Input|KeyboardEvents|DebugKeyPageDown
  (params (Key :type Key%20Structure :default "None") (ActionValue :type Input%20Action%20Value%20Structure))
  ;[0 0 0] Spawn item
  ;;[1 0.6921 0] DEBUG
  (:Pressed
    (bind _outrownames (DataTable|GetDataTableRowNames "/Game/Data/DataTable/DT_Furnitures.DT_Furnitures"))
    (Utilities|GetDataTableRow "/Game/Data/DataTable/DT_Furnitures.DT_Furnitures" (Utilities|Array|Get(acopy) _outrownames 20)
      (:then
        (bind _returnvalue (Game|SpawnActorfromClass "/Game/Blueprint/Gameplay/BP_Furniture.BP_Furniture_C" (Math|Transform|MakeTransform "0.000000,0.000000,250.000000" "0, 0, 0" "1.000000,1.000000,1.000000") "AlwaysSpawn" "MultiplyWithRoot" 0 (stale EventSpawnNewItem struct) 0))
        (Variables|Default|SetcurrentFurnitureRef _returnvalue)))))

(fn ConstructionScript
  (bind _dataasset (Variables|Default|GetdataAsset))
  (Camera|SetFieldOfView (Variables|Default|GetCineCamera) (Variables|/Game/Data/DataAsset/BP/BP_PlayerDA.BP_PlayerDA_C|GetbaseFOV _dataasset))
  (Variables|/Script/Engine.SpringArmComponent|SetTargetArmLength (Variables|Default|GetSpringArm) (Variables|/Game/Data/DataAsset/BP/BP_PlayerDA.BP_PlayerDA_C|GetcamDistanceBase _dataasset))
  (Transformation|SetRelativeRotation (Variables|Default|GetCineCamera) (Math|Rotator|MakeRotator 0.0 (* (Variables|/Game/Data/DataAsset/BP/BP_PlayerDA.BP_PlayerDA_C|GetcameraAngle _dataasset) -1.0) 0.0) false false)
  (Transformation|SetRelativeRotation (Variables|Default|GetSpringArm) (Math|Rotator|MakeRotator 0.0 (* (Variables|/Game/Data/DataAsset/BP/BP_PlayerDA.BP_PlayerDA_C|GetspringArmAngle _dataasset) -1.0) 0.0) false false)
  (Components|Timeline|SetPlayRate (Variables|Default|GetRotateCam) (Variables|/Game/Data/DataAsset/BP/BP_PlayerDA.BP_PlayerDA_C|GetrotationSpeed _dataasset)))

(fn OnRepCurrentFurnitureRef
  (Default|CallFurnitureChange (Variables|Default|GetcurrentFurnitureRef)))

(fn GetForwardfromMouse
  (params (length :type Float%20%28double-precision%29))
  (bind _returnvalue (Game|GetPlayerController 0))
  (bind _worldlocation (Game|Player|ConvertMouseLocationToWorldSpace _returnvalue))
  (return _worldlocation (+ _worldlocation (* (Math|Vector|GetForwardVector (Math|Rotator|FindLookatRotation (Camera|GetCameraLocation (Game|GetPlayerCameraManager 0)) (Transformation|GetWorldLocation (Variables|Default|GetWidget_Mouse)))) length))))

(fn GetPreviousHitActor
  (return (Variables|Default|GetpreviousHitActor)))