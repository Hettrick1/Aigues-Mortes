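; Menu preview actor that showcases random furniture from DT_WaitingFurnitures, with trilingual descriptions (FR/EN/DE) sent to the main menu widget.
; Once the widget reference is valid (polled), it picks a row and a left or right side, then normalizes mesh scale by bounds.
; One of two timeline macros animates it, either rotation or lateral drift.
; After a delay it asks the widget to fade out; StartMovement restarts the cycle.
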(event `self.ReceiveBeginPlay`
  (bind _randomboolvalue (`self.randomBoolValue`))
  (bind (_meshoffset_x _meshoffset_y _meshoffset_z) (`KismetMathLibrary.BreakVector` (`self.meshOffset`)))
  (bind _sm_item (`self.SM_Item`))
  (bind _dataassetref (`self.dataAssetRef`))
  (bind _meshoffset (`self.meshOffset`))
  (bind _dataassetref_2 (`self.dataAssetRef`))
  (bind _meshoffset_2 (`self.meshOffset`))
  (bind (_origin _boxextent) (`KismetSystemLibrary.GetComponentBounds` (`self.SM_Item`)))
  (bind (_returnvalue_x _returnvalue_y _returnvalue_z) (`KismetMathLibrary.BreakVector` (`SceneComponent.K2_GetComponentLocation` (`self.SM_Item`))))
  (bind (_returnvalue_x_2 _returnvalue_y_2 _returnvalue_z_2) (`KismetMathLibrary.BreakVector` (`SceneComponent.K2_GetComponentLocation` _sm_item)))
  (bind (_returnvalue_x_3 _returnvalue_y_3 _returnvalue_z_3) (`KismetMathLibrary.BreakVector` (`KismetMathLibrary.SelectVector` (+ (`/Game/Data/DataAsset/BP/BP_WaitingScreenDA.itemRightLocation` _dataassetref) _meshoffset) (+ _meshoffset (`/Game/Data/DataAsset/BP/BP_WaitingScreenDA.itemLeftLocation` _dataassetref)) (`self.meshRight`))))
  ;[0 0 0] Load Data Table
  (`/Engine/EditorBlueprintResources/StandardMacros.IsValid` (`self.mainMenuRef`) :!label _label
    (:`Is Valid`
      (`self.StopTimelines`)
      (set `self.meshRight` (>= (`/Game/Data/DataAsset/BP/BP_WaitingScreenDA.leftDisplayProbability` (`self.dataAssetRef`)) (`KismetMathLibrary.RandomFloatInRange` 0.0 1.0)))
      (bind _outrownames (`DataTableFunctionLibrary.GetDataTableRowNames` "/Game/Data/DataTable/DT_WaitingFurnitures.DT_WaitingFurnitures"))
      (bind _returnvalue (`|GetDataTableRow` "/Game/Data/DataTable/DT_WaitingFurnitures.DT_WaitingFurnitures" (`KismetArrayLibrary.Array_Random` _outrownames))
        (:`then`
          ;[0 0 0] ResetScales
          (`SceneComponent.SetRelativeScale3D` (`self.offset`) (1.0 1.0 1.0))
          (`SceneComponent.SetWorldScale3D` (`self.SM_Item`) (1.0 1.0 1.0))
          (bind (_highpolymesh _rotationoffset _scaleoffset _locationoffset _descriptionfr _descriptionen _descriptionde) (break `/Game/Data/Struct/S_WaitingFurniture` (`|Copy` _returnvalue)))
          ;[0 0 0] Set texts & mesh
          (`SceneComponent.K2_SetRelativeRotation` (`self.offset`) _rotationoffset false false)
          (`SceneComponent.SetRelativeScale3D` (`self.offset`) (`KismetMathLibrary.Conv_DoubleToVector` (+ 1.0 _scaleoffset)))
          (set `self.meshOffset` _locationoffset)
          (`/Game/Blueprint/UI/WBP_MainMenu.SetText` (`self.mainMenuRef`) (`|MakeArray` (`KismetTextLibrary.Conv_StringToText` _descriptionfr) (`KismetTextLibrary.Conv_StringToText` _descriptionen) (`KismetTextLibrary.Conv_StringToText` _descriptionde)) (not (`self.meshRight`)))
          (`StaticMeshComponent.SetStaticMesh` (`self.SM_Item`) _highpolymesh)
          (`SceneComponent.K2_SetWorldLocation` (`self.SM_Item`) (`KismetMathLibrary.SelectVector` (+ (`/Game/Data/DataAsset/BP/BP_WaitingScreenDA.itemRightLocation` _dataassetref_2) _meshoffset_2) (+ _meshoffset_2 (`/Game/Data/DataAsset/BP/BP_WaitingScreenDA.itemLeftLocation` _dataassetref_2)) (`self.meshRight`)) false false)
          (`SceneComponent.SetRelativeScale3D` (`self.SM_Item`) (* (/ 100.0 (`KismetMathLibrary.VSize` (`.BoxExtent` (`KismetSystemLibrary.GetComponentBounds` (`self.SM_Item`))))) (`SceneComponent.RelativeScale3D` (`self.offset`))))
          (`SceneComponent.K2_SetRelativeRotation` :`self` (`self.SM_Item`))
          (`|ExecutionSequence`
            (:`then_0`
              ;[0 0.5517 1] Play Random Anim
              (switch `int` (`KismetMathLibrary.RandomIntegerInRange` 0 1)
                (:`0`
                  (set `self.randomBoolValue` (`KismetMathLibrary.RandomBool`))
                  (set `self.randomFloatValue` (`KismetMathLibrary.SelectFloat` (`KismetMathLibrary.RandomFloatInRange` -20.0 -10.0) (`KismetMathLibrary.RandomFloatInRange` 10.0 20.0) (`KismetMathLibrary.RandomBool`)))
                  (set `self.zOffset` _returnvalue_z)
                  (bind (_direction _alpha) (`Timeline|rotate` :!via `PlayFromStart` :!label _label_2)
                    (:`Update`
                      (bind _returnvalue_2 (* _alpha (`self.randomFloatValue`)))
                      (bind _returnvalue_3 (* _returnvalue_2 0.5))
                      (`SceneComponent.K2_SetRelativeRotation` (`self.SM_Item`) (`KismetMathLibrary.MakeRotator` (`KismetMathLibrary.SelectFloat` _returnvalue_3 0.0 _randomboolvalue) (`KismetMathLibrary.SelectFloat` 0.0 _returnvalue_3 _randomboolvalue) _returnvalue_2) true false)
                      (`SceneComponent.K2_SetWorldLocation` _sm_item (`KismetMathLibrary.MakeVector` _returnvalue_x_2 _returnvalue_y_2 (`KismetMathLibrary.FInterpTo` _returnvalue_z_2 (+ (`self.zOffset`) (- 54.0 (.z (+ _origin (`KismetMathLibrary.MakeVector` 0.0 0.0 (* (.z _boxextent) -1.0)))) 100.0) _meshoffset_z) (`GameplayStatics.GetWorldDeltaSeconds`) 20.0)) false false))))
                (:`1`
                  (set `self.randomBoolValue` (`KismetMathLibrary.RandomBool`))
                  (bind (_direction_2 _alpha_2) (`Timeline|Timeline` :!via `PlayFromStart` :!label _label_3)
                    (:`Update`
                      (`SceneComponent.K2_SetWorldLocation` (`self.SM_Item`) (`KismetMathLibrary.MakeVector` (`KismetMathLibrary.Lerp` _returnvalue_x_3 (* _returnvalue_x_3 -1.0) (* _alpha_2 (`/Game/Data/DataAsset/BP/BP_WaitingScreenDA.LateralMovementMultiplyer` (`self.dataAssetRef`)))) _returnvalue_y_3 _returnvalue_z_3) false false)
                      (`SceneComponent.K2_SetRelativeRotation` (`self.SM_Item`) (* (`/Game/Data/DataAsset/BP/BP_WaitingScreenDA.latteralMovementRot` (`self.dataAssetRef`)) (* _alpha_2 (`KismetMathLibrary.SelectFloat` -1.0 1.0 (`self.randomBoolValue`)))) false false))))))
            (:`then_1`
              ;[0 0 0] Fade In Fade Out
              (`KismetSystemLibrary.Delay` (`/Game/Data/DataAsset/BP/BP_WaitingScreenDA.delayBetweenItems` (`self.dataAssetRef`)))
              (`/Game/Blueprint/UI/WBP_MainMenu.FadeOutEvent` (`self.mainMenuRef`) self))))))
    (:`Is Not Valid`
      (`KismetSystemLibrary.Delay` 0.1)
      (goto _label))))

(event `StartMovement`
  ;[0 0 0] Load Data Table
  (goto _label))

(event `StopTimelines`
  ;[0 0.5517 1] Play Random Anim
  (`|ExecutionSequence`
    (:`then_0`
      (goto _label_2 :!via `Stop`))
    (:`then_1`
      (goto _label_3 :!via `Stop`))))

(event `SetWidgetRef`
  (params (ref :type "/Game/Blueprint/UI/WBP_MainMenu Object Reference"))
  ;[0 0 0] SetWidgetRef
  (set `self.mainMenuRef` ref))

(fn `UserConstructionScript`)