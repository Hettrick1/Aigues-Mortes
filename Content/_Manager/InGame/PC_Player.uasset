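; Player controller that turns Enhanced Input actions for movement, camera, interaction, pause and furniture building into message calls on the player pawn.
; It switches between Player and Build mapping contexts, notifying the pawn of build mode.
; Most inputs restart a retriggerable AFK delay and dismiss any AFK widget, which is created on timeout with the HUD-dispatched language and a kick delay.
; A debug Backspace key toggles force feedback.
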(event Custom|ForceBuildMode
  (bind _returnvalue (PlayerController|LocalPlayerSubsystems|GetEnhancedInputLocalPlayerSubsystem))
  ;[1 1 1] Change mapping context
  (if (.ReturnValue (Class|EnhancedInputSubsystemInterface|HasMappingContext (PlayerController|LocalPlayerSubsystems|GetEnhancedInputLocalPlayerSubsystem) "/Game/_Manager/Input/Player/IMC_Player.IMC_Player"))
    (Input|RemoveMappingContext _returnvalue "/Game/_Manager/Input/Player/IMC_Player.IMC_Player" "(bIgnoreAllPressedKeysUntilRelease=True,bForceImmediately=False,bNotifyUserSettings=False)")
    (Input|AddMappingContext _returnvalue "/Game/_Manager/Input/Build/IMC_Build.IMC_Build" 0 "(bIgnoreAllPressedKeysUntilRelease=True,bForceImmediately=False,bNotifyUserSettings=False)")
    (Class|BPIPlayer|SetIsinBuildMode(Message) (Game|Player|GetPlayerPawn 0) true true)))

(event Custom|CheckInputTimer
  (bind _playerdataasset (Variables|Default|GetplayerDataAsset))
  ;[1 1 1] CheckAFKTimer
  (Utilities|FlowControl|Sequence
    (:then_0
      (Utilities|FlowControl|RetriggerableDelay (Variables|/Game/Data/DataAsset/BP/BP_PlayerDA.BP_PlayerDA_C|GetafkTime _playerdataasset))
      (bind _returnvalue (UserInterface|CreateWidget "/Game/Blueprint/UI/WBP_AFK_Player.WBP_AFK_Player_C" 0 (Variables|Default|Getlanguage) (Variables|/Game/Data/DataAsset/BP/BP_PlayerDA.BP_PlayerDA_C|GetafkDelayBeforeKick _playerdataasset)))
      (Variables|Default|SetafkWidget _returnvalue))
    (:then_1
      (Utilities|IsValid (Variables|Default|GetafkWidget)
        (:Is%20Valid
          (Class|CommonActivatableWidget|DeactivateWidget (Variables|Default|GetafkWidget))
          (Variables|Default|SetafkWidget 0))))))

(event Custom|SetPlayerLanguage
  (params (language :type Enum_Language%20Enum :default "NewEnumerator0"))
  ;[0 0 0] Bind language
  (Variables|Default|Setlanguage language))

(event Input|EnhancedActionEvents|EnhancedInputActionIA_Move
  (params (ActionValue :type Vector%202D%20Structure) (ElapsedSeconds :type Float%20%28double-precision%29) (TriggeredSeconds :type Float%20%28double-precision%29) (InputAction :type Input%20Action%20Object%20Reference :default "/Game/_Manager/Input/Player/IA/IA_Move.IA_Move"))
  ;[1 1 1] Move
  (:Triggered
    (Class|BPIPlayer|Move(Message) (Game|Player|GetPlayerPawn 0) ActionValue :!label _label)
    (CallFunction|CheckInputTimer))
  (:Canceled
    (goto _label))
  (:Completed
    (goto _label)))

(event Input|EnhancedActionEvents|EnhancedInputActionIA_Zoom
  (params (ActionValue :type Float%20%28double-precision%29) (ElapsedSeconds :type Float%20%28double-precision%29) (TriggeredSeconds :type Float%20%28double-precision%29) (InputAction :type Input%20Action%20Object%20Reference :default "/Game/_Manager/Input/Player/IA/IA_Zoom.IA_Zoom"))
  ;[1 1 1] Zoom
  (:Triggered
    (Class|BPIPlayer|Zoom(Message) (Game|Player|GetPlayerPawn 0) ActionValue :!label _label)
    (CallFunction|CheckInputTimer))
  (:Canceled
    (goto _label))
  (:Completed
    (goto _label)))

(event Input|EnhancedActionEvents|EnhancedInputActionIA_ChangeMode
  (params (ActionValue :type Boolean) (ElapsedSeconds :type Float%20%28double-precision%29) (TriggeredSeconds :type Float%20%28double-precision%29) (InputAction :type Input%20Action%20Object%20Reference :default "/Game/_Manager/Input/GlobalAction/IA_ChangeMode.IA_ChangeMode"))
  (bind _returnvalue (PlayerController|LocalPlayerSubsystems|GetEnhancedInputLocalPlayerSubsystem))
  (bind _returnvalue_2 (PlayerController|LocalPlayerSubsystems|GetEnhancedInputLocalPlayerSubsystem))
  ;[1 1 1] Change mapping context
  (:Started
    (CallFunction|CheckInputTimer)
    (if (.ReturnValue (Class|EnhancedInputSubsystemInterface|HasMappingContext _returnvalue_2 "/Game/_Manager/Input/Player/IMC_Player.IMC_Player"))
      (Input|RemoveMappingContext _returnvalue_2 "/Game/_Manager/Input/Player/IMC_Player.IMC_Player" "(bIgnoreAllPressedKeysUntilRelease=True,bForceImmediately=False,bNotifyUserSettings=False)")
      (Input|AddMappingContext _returnvalue "/Game/_Manager/Input/Build/IMC_Build.IMC_Build" 0 "(bIgnoreAllPressedKeysUntilRelease=True,bForceImmediately=False,bNotifyUserSettings=False)")
      (Class|BPIPlayer|SetIsinBuildMode(Message) (Game|Player|GetPlayerPawn 0) true false)
      (else
        (Input|RemoveMappingContext _returnvalue "/Game/_Manager/Input/Build/IMC_Build.IMC_Build" "(bIgnoreAllPressedKeysUntilRelease=True,bForceImmediately=False,bNotifyUserSettings=False)")
        (Input|AddMappingContext _returnvalue "/Game/_Manager/Input/Player/IMC_Player.IMC_Player" 0 "(bIgnoreAllPressedKeysUntilRelease=True,bForceImmediately=False,bNotifyUserSettings=False)")
        (Class|BPIPlayer|SetIsinBuildMode(Message) (Game|Player|GetPlayerPawn 0) false false)))))

(event Input|EnhancedActionEvents|EnhancedInputActionIA_RotateCam
  (params (ActionValue :type Vector%202D%20Structure) (ElapsedSeconds :type Float%20%28double-precision%29) (TriggeredSeconds :type Float%20%28double-precision%29) (InputAction :type Input%20Action%20Object%20Reference :default "/Game/_Manager/Input/Player/IA/IA_RotateCam.IA_RotateCam"))
  (:Triggered
    (Class|BPIPlayer|RotateCamera(Message) (Game|Player|GetPlayerPawn 0) (Math|Vector|MakeVector 0.0 (.y ActionValue) (.x ActionValue)) :!label _label))
  (:Completed
    (goto _label)))

(event Input|EnhancedActionEvents|EnhancedInputActionIA_ChangeVariant
  (params (ActionValue :type Boolean) (ElapsedSeconds :type Float%20%28double-precision%29) (TriggeredSeconds :type Float%20%28double-precision%29) (InputAction :type Input%20Action%20Object%20Reference :default "/Game/_Manager/Input/Build/Actions/IA_ChangeVariant.IA_ChangeVariant"))
  ;[1 1 1] Build mode
  (:Started
    (Class|BPIPlayer|ChangeVariant(Message) (Game|Player|GetPlayerPawn 0))
    (CallFunction|CheckInputTimer)))

(event Input|EnhancedActionEvents|EnhancedInputActionIA_Interact
  (params (ActionValue :type Boolean) (ElapsedSeconds :type Float%20%28double-precision%29) (TriggeredSeconds :type Float%20%28double-precision%29) (InputAction :type Input%20Action%20Object%20Reference :default "/Game/_Manager/Input/Player/IA/IA_Interact.IA_Interact"))
  ;[1 1 1] Interact
  (:Started
    (Class|BPIPlayer|Interact(Message) (Game|Player|GetPlayerPawn 0))
    (CallFunction|CheckInputTimer)))

(event Input|EnhancedActionEvents|EnhancedInputActionIA_QuestRecap
  (params (ActionValue :type Boolean) (ElapsedSeconds :type Float%20%28double-precision%29) (TriggeredSeconds :type Float%20%28double-precision%29) (InputAction :type Input%20Action%20Object%20Reference :default "/Game/_Manager/Input/GlobalAction/IA_QuestRecap.IA_QuestRecap"))
  ;[1 1 1] Pause
  (:Started
    (Class|BPIPlayer|Pause(Message) (Game|Player|GetPlayerPawn 0))
    (CallFunction|CheckInputTimer)))

(event Input|EnhancedActionEvents|EnhancedInputActionIA_Rotate
  (params (ActionValue :type Float%20%28double-precision%29) (ElapsedSeconds :type Float%20%28double-precision%29) (TriggeredSeconds :type Float%20%28double-precision%29) (InputAction :type Input%20Action%20Object%20Reference :default "/Game/_Manager/Input/Player/IA/IA_Rotate.IA_Rotate"))
  ;[1 1 1] Rotate
  (:Started
    (Class|BPIPlayer|Rotate(Message) (Game|Player|GetPlayerPawn 0) (Math|Float|Truncate ActionValue))
    (CallFunction|CheckInputTimer)))

(event Input|EnhancedActionEvents|EnhancedInputActionIA_MoveFurniture
  (params (ActionValue :type Vector%202D%20Structure) (ElapsedSeconds :type Float%20%28double-precision%29) (TriggeredSeconds :type Float%20%28double-precision%29) (InputAction :type Input%20Action%20Object%20Reference :default "/Game/_Manager/Input/Build/Actions/IA_MoveFurniture.IA_MoveFurniture"))
  (bind _returnvalue (Game|Player|GetPlayerPawn 0))
  ;[1 1 1] Build mode
  (:Triggered
    (Class|BPIPlayer|MoveFurniture(Message) _returnvalue ActionValue TriggeredSeconds)
    (CallFunction|CheckInputTimer :!label _label))
  (:Completed
    (Class|BPIPlayer|StopMovingFurniture(Message) _returnvalue TriggeredSeconds)
    (goto _label)))

(event Input|EnhancedActionEvents|EnhancedInputActionIA_MouseMovement
  (params (ActionValue :type Vector%202D%20Structure) (ElapsedSeconds :type Float%20%28double-precision%29) (TriggeredSeconds :type Float%20%28double-precision%29) (InputAction :type Input%20Action%20Object%20Reference :default "/Game/_Manager/Input/Build/Actions/IA_MouseMovement.IA_MouseMovement"))
  (Class|BPIPlayer|MoveMouse(Message) (Game|Player|GetPlayerPawn 0) ActionValue)
  (CallFunction|CheckInputTimer))

(event Input|EnhancedActionEvents|EnhancedInputActionIA_RotateFurniture
  (params (ActionValue :type Float%20%28double-precision%29) (ElapsedSeconds :type Float%20%28double-precision%29) (TriggeredSeconds :type Float%20%28double-precision%29) (InputAction :type Input%20Action%20Object%20Reference :default "/Game/_Manager/Input/Build/Actions/IA_RotateFurniture.IA_RotateFurniture"))
  ;[1 1 1] Build mode
  (:Started
    (Class|BPIPlayer|RotateFurniture(Message) (Game|Player|GetPlayerPawn 0) (Math|Float|Round ActionValue))))

(event Input|EnhancedActionEvents|EnhancedInputActionIA_PlaceFurniture
  (params (ActionValue :type Boolean) (ElapsedSeconds :type Float%20%28double-precision%29) (TriggeredSeconds :type Float%20%28double-precision%29) (InputAction :type Input%20Action%20Object%20Reference :default "/Game/_Manager/Input/Build/Actions/IA_PlaceFurniture.IA_PlaceFurniture"))
  ;[1 1 1] Build mode
  (:Started
    (Class|BPIPlayer|AcceptFurniture(Message) (Game|Player|GetPlayerPawn 0))
    (CallFunction|CheckInputTimer)))

(event Input|EnhancedActionEvents|EnhancedInputActionIA_CancelPlacing
  (params (ActionValue :type Boolean) (ElapsedSeconds :type Float%20%28double-precision%29) (TriggeredSeconds :type Float%20%28double-precision%29) (InputAction :type Input%20Action%20Object%20Reference :default "/Game/_Manager/Input/Build/Actions/IA_CancelPlacing.IA_CancelPlacing"))
  ;[1 1 1] Build mode
  (:Started
    (Class|BPIPlayer|CancelFurniture(Message) (Game|Player|GetPlayerPawn 0))
    (CallFunction|CheckInputTimer)))

(event EventBeginPlay
  (bind _returnvalue (PlayerController|LocalPlayerSubsystems|GetEnhancedInputLocalPlayerSubsystem))
  ;[1 0 0] Add mapping Context
  (Utilities|IsValid _returnvalue
    (:Is%20Valid
      (Input|AddMappingContext _returnvalue "/Game/_Manager/Input/Player/IMC_Player.IMC_Player" 0 "(bIgnoreAllPressedKeysUntilRelease=True,bForceImmediately=False,bNotifyUserSettings=False)")
      ;[0 0 0] Bind language
      (EventDispatchers|BindEventtoSetLanguageDispatcher (.AsHUD%20Game (Utilities|Casting|CastToHUD_Game (HUD|GetHUD))) (delegate Custom|SetPlayerLanguage)))))

(event Input|KeyboardEvents|DebugKeyBackspace
  (params (Key :type Key%20Structure) (ActionValue :type Input%20Action%20Value%20Structure))
  ;[1 0.6841 0] DEBUG ONLY
  (:Pressed
    (Utilities|FlowControl|FlipFlop
      (:A
        (Variables|Default|SetbForceFeedbackEnabled false))
      (:B
        (Variables|Default|SetbForceFeedbackEnabled true)))))

(fn ConstructionScript)