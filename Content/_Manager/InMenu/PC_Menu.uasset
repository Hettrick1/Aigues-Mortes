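; Player controller for the main menu, handling input to start the game and show or hide the credits.
; BeginPlay adds the menu Enhanced Input mapping context, and the start action opens the game map when CanStartGame is set.
; A FlipFlop alternates between adding credits through HUD_MainMenu and calling CallCloseCredit, tracking CreditsOpen so Go Back only triggers it to close.
; A disconnected waiting-screen tutorial branch never runs.
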(event `self.ReceiveBeginPlay`
  (bind _returnvalue (subsystem `EnhancedInputLocalPlayerSubsystem`))
  ;[1 0 0] Add mapping Context
  (`/Engine/EditorBlueprintResources/StandardMacros.IsValid` _returnvalue
    (:`Is Valid`
      (message `EnhancedInputSubsystemInterface.AddMappingContext` _returnvalue "/Game/_Manager/Input/Menu/IMC_Menu.IMC_Menu" 0 (struct)))))

(event `EnhancedInput|/Game/_Manager/Input/Menu/IA_StartGame`
  (params (ActionValue :type Boolean) (ElapsedSeconds :type "Float (double-precision)") (TriggeredSeconds :type "Float (double-precision)") (InputAction :type "InputAction Object Reference" :default "/Game/_Manager/Input/Menu/IA_StartGame.IA_StartGame"))
  (:`Started`
    (if (`self.canStartGame`)
      (`GameplayStatics.OpenLevelBySoftObjectPtr` "/Game/Level/LVL_GameMap.LVL_GameMap"))))

(event `EnhancedInput|/Game/_Manager/Input/Menu/IA_Credit`
  (params (ActionValue :type Boolean) (ElapsedSeconds :type "Float (double-precision)") (TriggeredSeconds :type "Float (double-precision)") (InputAction :type "InputAction Object Reference" :default "/Game/_Manager/Input/Menu/IA_Credit.IA_Credit"))
  (:`Started`
    (bind _isa (`/Engine/EditorBlueprintResources/StandardMacros.FlipFlop` :!label _label)
      (:`A`
        (`/Game/Blueprint/_BPI/BPI_HUD.AddCredit` (cast `/Game/_Manager/InMenu/HUD_MainMenu` (`self.GetHUD`) :!pure true))
        (set `self.creditsOpen` _isa))
      (:`B`
        (`self.CloseCredit`)
        (set `self.creditsOpen` _isa)))))

(event `EnhancedInput|/Game/_Manager/Input/Menu/IA_GoBack`
  (params (ActionValue :type Boolean) (ElapsedSeconds :type "Float (double-precision)") (TriggeredSeconds :type "Float (double-precision)") (InputAction :type "InputAction Object Reference" :default "/Game/_Manager/Input/Menu/IA_GoBack.IA_GoBack"))
  (:`Started`
    (if (`self.creditsOpen`)
      (goto _label))))

(fn `UserConstructionScript`)