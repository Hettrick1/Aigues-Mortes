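; BP_Player is the player character Blueprint, handling movement, camera look, pausing and a still-empty Interract event.
; Move stores the input magnitude in MovementVelocity and adds movement relative to control yaw.
; Look sends yaw to the controller but pitches the SpringArm directly, clamped short of vertical.
; Pause messages the HUD to add WBP_PauseMenu.
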(event `/Game/Blueprints/BPI/BPI_Player.Move`
  (params (axis :type "Vector2D Structure"))
  (bind (_x _y) (`KismetMathLibrary.BreakVector2D` axis))
  (bind (_returnvalue_roll _returnvalue_pitch _returnvalue_yaw) (`KismetMathLibrary.BreakRotator` (`self.GetControlRotation`)))
  (bind _returnvalue (`KismetMathLibrary.MakeRotator` _returnvalue_roll 0.0 _returnvalue_yaw))
  ;[1 1 1] MovePlayer
  (set `self.movementVelocity` (`KismetMathLibrary.VSize2D` axis))
  (`self.AddMovementInput` (`KismetMathLibrary.GetForwardVector` _returnvalue) _y)
  (`self.AddMovementInput` (`KismetMathLibrary.GetRightVector` _returnvalue) _x))

(event `/Game/Blueprints/BPI/BPI_Player.Look`
  (params (axis :type "Vector2D Structure"))
  (bind (_x _y) (`KismetMathLibrary.BreakVector2D` axis))
  (bind _springarm (`self.SpringArm`))
  (bind (_relativerotation_roll _relativerotation_pitch _relativerotation_yaw) (`KismetMathLibrary.BreakRotator` (`SceneComponent.RelativeRotation` _springarm)))
  ;[1 1 1] Rotate Camera
  (`self.AddControllerYawInput` _x)
  (`SceneComponent.K2_SetRelativeRotation` _springarm (`KismetMathLibrary.MakeRotator` _relativerotation_roll (`KismetMathLibrary.FClamp` (+ (* _y -1.0) _relativerotation_pitch) -89.0 89.0) _relativerotation_yaw) false false))

(event `/Game/Blueprints/BPI/BPI_Player.Interract`
  ;[1 1 1] Interract
)

(event `/Game/Blueprints/BPI/BPI_Player.Pause`
  ;[1 1 1] Pause
  (message `/Game/Blueprints/BPI/BPI_HUD.AddWidget` (`PlayerController.GetHUD` (`GameplayStatics.GetPlayerController` 0)) "/Game/Blueprints/UI/WBP_PauseMenu.WBP_PauseMenu_C" false))

(fn `UserConstructionScript`
  (`parent.UserConstructionScript`))